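; Game mode that holds the score and the rule for when the bomb explodes.
; On BeginPlay it creates the Name widget and adds it to the viewport.
; Every Tick it counts all BP_Light actors in the level and sets Exploding once that count equals PassedLight.
; AddScore increments TotalScore by one; PassedLight is only read here, never updated.
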(event `self.ReceiveBeginPlay`
  ;[1 1 1] 뷰포트에 탑재
  (bind _returnvalue (`|CreateWidget` "/Game/UI/Name.Name_C"))
  (`UserWidget.AddToViewport` _returnvalue 0))

(event `self.ReceiveTick`
  (params (DeltaSeconds :type "Float (single-precision)"))
  ;[1 1 1] 폭탄이 폭발하는 게임 규칙
  (bind _outactors (`GameplayStatics.GetAllActorsOfClass` "/Game/Blueprints/BP_Light.BP_Light_C"))
  (bind _output_get (set `self.NumbersOfLight` (`KismetArrayLibrary.Array_Length` _outactors)))
  (if (== _output_get (`self.PassedLight`))
    (set `self.Exploding` true)))

(fn `Add Score`
  (set `self.TotalScore` (+ (`self.TotalScore`) 1)))

(fn `UserConstructionScript`)