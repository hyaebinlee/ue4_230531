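; BP_Light is a light actor that switches on when something first overlaps its trigger and counts as a passed light.
; The Box overlap runs through a DoOnce, sets the Lighting flag and increments PassedLight on BP_MyGameMode, without filtering which actor overlapped.
; Tick applies the Lighting flag to the PointLight's visibility every frame.
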(event `self.ReceiveTick`
  (params (DeltaSeconds :type "Float (single-precision)"))
  ;[1 1 1] 캐릭터가 일정 범위에 들어오면 불이 켜짐
  (`SceneComponent.SetVisibility` (`self.PointLight`) (`self.Lighting`) false))

(event `self.Box.OnComponentBeginOverlap`
  (params (OverlappedComponent :type "PrimitiveComponent Object Reference") (OtherActor :type "Actor Object Reference") (OtherComp :type "PrimitiveComponent Object Reference") (OtherBodyIndex :type Integer) (bFromSweep :type Boolean) (SweepResult :type "HitResult Structure (by ref)"))
  ;[1 1 1] 액터끼리 접촉하는 순간에 불이 지고 카운트
  (`/Engine/EditorBlueprintResources/StandardMacros.DoOnce` false
    (:`Completed`
      (set `self.Lighting` true)
      (bind _asbp_my_game_mode (cast `/Game/Blueprints/BP_MyGameMode` (`GameplayStatics.GetGameMode`)))
      (set `/Game/Blueprints/BP_MyGameMode.PassedLight` (+ (`/Game/Blueprints/BP_MyGameMode.PassedLight` _asbp_my_game_mode) 1) _asbp_my_game_mode))))

(fn `UserConstructionScript`)